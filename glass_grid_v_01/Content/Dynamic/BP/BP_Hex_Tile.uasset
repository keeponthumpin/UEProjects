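; Hex tile actor that plays a MIDI note and animates its glow, color and height when something overlaps its trigger.
; BeginPlay picks a random height and creates a dynamic glass material.
; Overlap sends Note On and runs timelines that drive emissive and RGB-scaled color parameters, ease tile Z scale between that height and one, and stretch the trigger.
; End overlap runs a timeline that sends Note Off every update with the curve as velocity.
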(event OnComponentBeginOverlap(HexTrigger)
  (params (OverlappedComponent :type Primitive%20Component%20Object%20Reference) (OtherActor :type Actor%20Object%20Reference) (OtherComp :type Primitive%20Component%20Object%20Reference) (OtherBodyIndex :type Integer) (bFromSweep :type Boolean) (SweepResult :type Hit%20Result%20Structure%20%28by%20ref%29))
  (bind _rgb (Variables|Default|GetRGB))
  (bind _randomheight (Variables|Default|GetRandomHeight))
  (bind (_x _y _z) (Math|Vector|BreakVector _rgb))
  (Class|MIDIDeviceOutputController|SendMIDINoteon (Variables|Default|GetMidiDevice) (Variables|Default|GetChannel) (Variables|Default|GetNote) (Variables|Default|GetVelocity))
  (Utilities|FlowControl|Sequence
    (:then_0
      (bind _newtrack_0 (Timeline|Emissive PlayFromStart)
        (:Update
          (Rendering|Material|SetScalarParameterValue (Variables|Default|GetMaterial) "Emissive" _newtrack_0 :!class /Script/Engine.MaterialInstanceDynamic))))
    (:then_1
      (bind _newtrack_0_2 (Timeline|Color_1 PlayFromStart)
        (:Update
          (Rendering|Material|SetScalarParameterValue (Variables|Default|GetMaterial) "R" (* _newtrack_0_2 _x) :!class /Script/Engine.MaterialInstanceDynamic))))
    (:then_2
      (bind _newtrack_0_3 (Timeline|Color_2 PlayFromStart)
        (:Update
          (Rendering|Material|SetScalarParameterValue (Variables|Default|GetMaterial) "G" (* _newtrack_0_3 _y) :!class /Script/Engine.MaterialInstanceDynamic))))
    (:then_3
      (bind _newtrack_0_4 (Timeline|Color_3 PlayFromStart)
        (:Update
          (Rendering|Material|SetScalarParameterValue (Variables|Default|GetMaterial) "B" (* _newtrack_0_4 _z) :!class /Script/Engine.MaterialInstanceDynamic))))
    (:then_4
      (bind _newtrack_0_5 (Timeline|Timeline_3 Play)
        (:Update
          (Transformation|SetWorldScale3D (Variables|Default|GetHexTile) (Math|Vector|MakeVector 1.0 1.0 (Math|Interpolation|Ease "Linear" _newtrack_0_5 _randomheight 1.0)))
          (Transformation|SetWorldScale3D (Variables|Default|GetHexTrigger) (Math|Vector|MakeVector 1.0 1.0 (+ _randomheight 5.0))))))))

(event OnComponentEndOverlap(HexTrigger)
  (params (OverlappedComponent :type Primitive%20Component%20Object%20Reference) (OtherActor :type Actor%20Object%20Reference) (OtherComp :type Primitive%20Component%20Object%20Reference) (OtherBodyIndex :type Integer))
  (bind _newtrack_0 (Timeline|Timeline Play)
    (:Update
      (Class|MIDIDeviceOutputController|SendMIDINoteOff (Variables|Default|GetMidiDevice) (Variables|Default|GetChannel) (Variables|Default|GetNote) (Math|Float|Truncate _newtrack_0)))))

(event EventBeginPlay
  (Utilities|FlowControl|Sequence
    (:then_0
      (Variables|Default|SetRandomHeight (Math|Random|RandomFloatinRange 1.0 1e+01)))
    (:then_1
      (bind _returnvalue (Rendering|Material|CreateDynamicMaterialInstance (Variables|Default|GetHexTile) 0 "/Game/Static/M_glass.M_glass" "None" :!class /Script/Engine.PrimitiveComponent))
      (Variables|Default|SetMaterial _returnvalue))))

(fn ConstructionScript)