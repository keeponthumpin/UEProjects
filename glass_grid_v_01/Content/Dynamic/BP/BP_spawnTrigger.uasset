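; BP_spawnTrigger is an actor that lays out a test grid of box components, with no gameplay logic in its event graph.
; When SpawnTestGrid is set, the construction script loops over GridX and GridY and adds a box at each spacing-based position.
; Every odd X column is shifted along Y by Offset, producing a staggered pattern.
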(event EventBeginPlay)

(event Collision|EventActorBeginOverlap
  (params (OtherActor :type Actor%20Object%20Reference)))

(event EventTick
  (params (DeltaSeconds :type Float%20%28single-precision%29)))

(fn ConstructionScript
  (if (Variables|Default|GetSpawnTestGrid)
    (for _index (range 0 (Variables|Default|GetGridX))
      (for _index_2 (range 0 (Variables|Default|GetGridY))
        (AddComponent|AddBoxComponent false (Math|Transform|MakeTransform (Math|Vector|SelectVector (Math|Vector|MakeVector (* _index (Variables|Default|GetSpacingX)) (* _index_2 (Variables|Default|GetSpaсingY)) 0.0) (Math|Vector|MakeVector (* _index (Variables|Default|GetSpacingX)) (+ (Variables|Default|GetOffset) (* _index_2 (Variables|Default|GetSpaсingY))) 0.0) (== (Math|Integer|%(Integer) _index 2) 0)) "0, 0, 0" "1.000000,1.000000,1.000000"))))))