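; Actor that generates a hex grid of BP_Hex_Tile actors, each assigned a random MIDI note and a color.
; On BeginPlay it repositions the third-person character, opens a MIDI output matching DeviceName and loads notes from a data table.
; Tiles spawn with alternate columns offset, receiving the MIDI device and an HSV-derived hue mapped to the note's range.
; Optionally, the construction script builds a test grid of randomly tall static mesh components.
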(event EventBeginPlay
  (bind _notes_array (Variables|Default|GetNotes%20Array))
  (bind _minvalue (Math|Integer|MinOfIntArray _notes_array))
  (Utilities|FlowControl|Sequence
    (:then_0
      (CallFunction|SetPlayerActorLocation)
      (CallFunction|CreateMidiDevice)
      (CallFunction|GetNotesfromTable)
      (for _index (range 0 (Variables|Default|GetGridX))
        (for _index_2 (range 0 (Variables|Default|GetGridY))
          (bind _returnvalue (Game|SpawnActorfromClass "/Game/Dynamic/BP/BP_Hex_Tile.BP_Hex_Tile_C" (Math|Transform|MakeTransform (Math|Vector|SelectVector (Math|Vector|MakeVector (* _index (Variables|Default|GetSpacingX)) (* _index_2 (Variables|Default|GetSpasingY)) 0.0) (Math|Vector|MakeVector (* _index (Variables|Default|GetSpacingX)) (+ (* _index_2 (Variables|Default|GetSpasingY)) (Variables|Default|GetOffset)) 0.0) (== (Math|Integer|%(Integer) _index 2) 0)) "0, 0, 0" (Math|Vector|MakeVector 1.0 1.0 1.0)) "Undefined" "MultiplyWithRoot" 0 0))
          (bind _output_get (Variables|/Game/Dynamic/BP/BP_Hex_Tile.BP_Hex_Tile_C|SetNote _returnvalue (.OutItem (Utilities|Array|Random (Variables|Default|GetNotes%20Array)))))
          (Variables|/Game/Dynamic/BP/BP_Hex_Tile.BP_Hex_Tile_C|SetMidiDevice _returnvalue (Variables|Default|GetMidi%20Device%20Output))
          (Variables|/Game/Dynamic/BP/BP_Hex_Tile.BP_Hex_Tile_C|SetRGB _returnvalue (Math|Vector|MakeVector (.r (Class|KismetMathLibrary|HSVtoRGB (* (/ (Math|Conversions|ToFloat(Integer) (- _output_get _minvalue)) (Math|Conversions|ToFloat(Integer) (- (.MaxValue (Math|Integer|MaxOfIntArray _notes_array)) _minvalue))) 3.5e+02) 1.0 1.0 0.0)) (.g (Class|KismetMathLibrary|HSVtoRGB (* (/ (Math|Conversions|ToFloat(Integer) (- _output_get _minvalue)) (Math|Conversions|ToFloat(Integer) (- (.MaxValue (Math|Integer|MaxOfIntArray _notes_array)) _minvalue))) 3.5e+02) 1.0 1.0 0.0)) (.b (Class|KismetMathLibrary|HSVtoRGB (* (/ (Math|Conversions|ToFloat(Integer) (- _output_get _minvalue)) (Math|Conversions|ToFloat(Integer) (- (.MaxValue (Math|Integer|MaxOfIntArray _notes_array)) _minvalue))) 3.5e+02) 1.0 1.0 0.0)))))))))

(event Collision|EventActorBeginOverlap
  (params (OtherActor :type Actor%20Object%20Reference)))

(event EventTick
  (params (DeltaSeconds :type Float%20%28single-precision%29)))

(fn ConstructionScript
  (if (Variables|Default|GetSpawnTestGrid)
    (for _index (range 0 (Variables|Default|GetGridX))
      (for _index_2 (range 0 (Variables|Default|GetGridY))
        (bind _returnvalue (AddComponent|AddStaticMeshComponent false (Math|Transform|MakeTransform (Math|Vector|SelectVector (Math|Vector|MakeVector (* _index (Variables|Default|GetSpacingX)) (* _index_2 (Variables|Default|GetSpasingY)) 0.0) (Math|Vector|MakeVector (* _index (Variables|Default|GetSpacingX)) (+ (Variables|Default|GetOffset) (* _index_2 (Variables|Default|GetSpasingY))) 0.0) (== (Math|Integer|%(Integer) _index 2) 0)) "0, 0, 0" "1.000000,1.000000,1.000000")))
        (Transformation|SetWorldScale3D _returnvalue (Math|Vector|MakeVector 1.0 1.0 (Math|Random|RandomFloatinRange 1.0 1e+01)))))))

(fn GetNotesfromTable
  (Utilities|Array|Clear (Variables|Default|GetNotes%20Array))
  (bind _outrownames (DataTable|GetDataTableRowNames (Variables|Default|GetTable)))
  (for _array_element _outrownames
    (bind _returnvalue (Utilities|GetDataTableRow (Variables|Default|GetTable) _array_element)
      (:then
        (Utilities|Array|Add (Variables|Default|GetNotes%20Array) (Math|Conversions|ToInteger(Byte) (Utilities|Struct|BreakStruct_Notes _returnvalue)))))))

(fn SetPlayerActorLocation
  (bind _returnvalue (Actor|GetActorOfClass "/Game/ThirdPerson/Blueprints/BP_ThirdPersonCharacter.BP_ThirdPersonCharacter_C"))
  (Transformation|SetActorLocation _returnvalue (Math|Vector|MakeVector (Math|Conversions|ToFloat(Integer) (* (Variables|Default|GetGridX) 20)) (Math|Conversions|ToFloat(Integer) (* (Variables|Default|GetGridY) 20)) 3e+02) false true)
  (Development|PrintString "Hello"))

(fn CreateMidiDevice
  (bind _devices_ids_array (Variables|Default|GetDevices%20IDs%20Array))
  (bind _outmididevices (Class|MIDIDeviceManager|FindMIDIDevices))
  (for _array_element _outmididevices
    (Utilities|FlowControl|Sequence
      (:then_0
        (if (Utilities|Enum|Equal(Enum) (.DeviceName (Utilities|Struct|BreakFoundMIDIDevice _array_element)) (Variables|Default|GetDeviceName))
          (Utilities|Array|Add _devices_ids_array (.DeviceID (Utilities|Struct|BreakFoundMIDIDevice _array_element)))
          (bind _output_get (Variables|Default|SetDevice%20ID (Utilities|Array|Get(acopy) _devices_ids_array (Utilities|Array|LastIndex _devices_ids_array))))
          (bind _returnvalue (Class|MIDIDeviceManager|CreateMIDIDeviceOutputController _output_get))
          (Utilities|IsValid _returnvalue
            (:Is%20Valid
              (Variables|Default|SetMidi%20Device%20Output _returnvalue))))))))