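; Spawner actor that creates a diagonal row of BP_Bounce balls, one per note in the DonnaLee data table, for MIDI output.
; On BeginPlay it opens a MIDI output controller for the device matching DeviceName, then reads the table's notes into an array.
; Each ball is offset in X and Z by index and receives the controller, its note, a stepped velocity and an emissive color.
; DeviceNameChanged reruns only the MIDI setup.
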(event Custom|DeviceNameChanged
  (CallFunction|MIDIOutputcontrollerSetup))

(event EventBeginPlay
  (Utilities|FlowControl|Sequence
    (:then_0
      (CallFunction|MIDIOutputcontrollerSetup))
    (:then_1
      (CallFunction|CreateNotesArrayfromDataTable))
    (:then_2
      (for _index (range 0 (- (Utilities|Array|Length (Variables|Default|GetNotes%20Array)) 1))
        (bind (_returnvalue _outputpin) (CallFunction|CreateBallsTransfroms _index _index _index))
        (CallFunction|SetBallsParameters _index _returnvalue _outputpin)))))

(fn ConstructionScript)

(fn MIDIOutputcontrollerSetup
  (bind _devices_ids_array (Variables|Default|GetDevices%20IDs%20Array))
  ;[1 1 1] 1. Find all of the devices. 2.Find device which name matches the midi output we are using. 3. Setup MIDI Output Controller with device ID from the step 2.
  (bind _outmididevices (Class|MIDIDeviceManager|FindMIDIDevices))
  (for _array_element _outmididevices
    (Utilities|FlowControl|Sequence
      (:then_0
        (if (Utilities|Enum|Equal(Enum) (.DeviceName (Utilities|Struct|BreakFoundMIDIDevice _array_element)) (Variables|Default|GetDeviceName))
          (Utilities|Array|Add _devices_ids_array (.DeviceID (Utilities|Struct|BreakFoundMIDIDevice _array_element)))
          (bind _output_get (Variables|Default|SetDevice%20ID (Utilities|Array|Get(acopy) _devices_ids_array (Utilities|Array|LastIndex _devices_ids_array))))
          (bind _returnvalue (Class|MIDIDeviceManager|CreateMIDIDeviceOutputController _output_get))
          (Utilities|IsValid _returnvalue
            (:Is%20Valid
              (Variables|Default|SetMidi%20Device%20Output _returnvalue)))))
      (:then_1
        (Utilities|Array|Add (Variables|Default|GetDevices%20Array) (Utilities|String|ToString(Text) (Utilities|Text|FormatText "{Device name} " (.DeviceName (Utilities|Struct|BreakFoundMIDIDevice _array_element)))))))))

(fn CreateNotesArrayfromDataTable
  (bind _outrownames (DataTable|GetDataTableRowNames "/Game/DonnaLee.DonnaLee"))
  (for _array_element _outrownames
    (bind _returnvalue (Utilities|GetDataTableRow "/Game/DonnaLee.DonnaLee" _array_element)
      (:then
        (Utilities|Array|Add (Variables|Default|GetNotes%20Array) (Math|Conversions|ToInteger(Byte) (Utilities|Struct|BreakStruct_Notes _returnvalue)))))))

(fn CreateBallsTransfroms
  (params (InputPin :type Integer) (A :type Integer) (A2 :type Integer))
  (bind _returnvalue (Transformation|GetActorTransform))
  (bind (_location _rotation _scale) (Math|Transform|BreakTransform _returnvalue))
  (bind (_x _y _z) (Math|Vector|BreakVector _location))
  (return (Math|Transform|MakeTransform (Math|Vector|MakeVector (+ _x (* A2 (Variables|Default|GetDistanceX))) _y (+ _z (* A (Variables|Default|GetDistanceZ)))) _rotation _scale) InputPin))

(fn SetBallsParameters
  (params (InputPin :type Integer) (SpawnTransform :type Transform) (InputPin2 :type Integer))
  (bind _returnvalue (Game|SpawnActorfromClass "/Game/Dynamic/BPs/BP_Bounce.BP_Bounce_C" SpawnTransform "Undefined" "MultiplyWithRoot" 0 0))
  ;[1 1 1] Set spawned balls colors
  (Rendering|Material|SetVectorParameterValue (Variables|/Game/Dynamic/BPs/BP_Bounce.BP_Bounce_C|GetM_Glow _returnvalue) "EmissiveColor" (Variables|Default|GetEmissiveColor) :!class /Script/Engine.MaterialInstanceDynamic)
  (Variables|/Game/Dynamic/BPs/BP_Bounce.BP_Bounce_C|SetPrintValues _returnvalue (Variables|Default|GetDebug%20Output))
  (Variables|/Game/Dynamic/BPs/BP_Bounce.BP_Bounce_C|SetMidiDeviceOutput _returnvalue (Variables|Default|GetMidi%20Device%20Output))
  (Variables|/Game/Dynamic/BPs/BP_Bounce.BP_Bounce_C|SetNote _returnvalue (Utilities|Array|Get(acopy) (Variables|Default|GetNotes%20Array) InputPin))
  (Variables|/Game/Dynamic/BPs/BP_Bounce.BP_Bounce_C|SetVelocity _returnvalue (+ (* InputPin2 (Variables|Default|GetVelocity%20Increment)) (Variables|Default|GetVelocity%20Start))))