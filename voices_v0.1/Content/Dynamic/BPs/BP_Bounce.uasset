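; BP_Bounce is an actor that sends a MIDI Note On whenever another actor overlaps it, using its channel, note and velocity variables.
; Each hit also plays a timeline that drives emission on the SphereGoal's dynamic material, with optional printing of the sent values.
; A SetDeviceName function resolves a MIDI device ID by name, but nothing in these graphs calls it.
; No Note Off is sent.
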(event Collision|EventActorBeginOverlap
  (params (OtherActor :type Actor%20Object%20Reference))
  (Class|MIDIDeviceOutputController|SendMIDINoteon (Variables|Default|GetMidiDeviceOutput) (Variables|Default|GetChannel) (Variables|Default|GetNote) (Variables|Default|GetVelocity))
  (Utilities|FlowControl|Sequence
    (:then_0
      (if (Variables|Default|GetPrintValues)
        (CallFunction|PrintOutcomingValues)))
    (:then_1
      (bind _newtrack_0 (Timeline|Timeline PlayFromStart)
        (:Update
          (Rendering|Material|SetScalarParameterValue (Variables|Default|GetM_Glow) "EmissionMult" (* _newtrack_0 (+ (Variables|Default|GetGlowAmount) 2e+02)) :!class /Script/Engine.MaterialInstanceDynamic))))))

(event EventBeginPlay
  (bind _returnvalue (Rendering|Material|CreateDynamicMaterialInstance (Variables|Default|GetSphereGoal) 0 "/Game/Static/Materials/M_Emissive_Inst.M_Emissive_Inst" "None" :!class /Script/Engine.PrimitiveComponent))
  (Variables|Default|SetM_Glow _returnvalue))

(fn ConstructionScript)

(fn SetDeviceName
  (bind _devices_ids_array (Variables|Default|GetDevices%20IDs%20Array))
  (bind _outmididevices (Class|MIDIDeviceManager|FindMIDIDevices))
  (for _array_element _outmididevices
    (if (Utilities|Enum|Equal(Enum) (.DeviceName (Utilities|Struct|BreakFoundMIDIDevice _array_element)) (Variables|Default|GetDeviceName))
      (Utilities|Array|Add (Variables|Default|GetDevices%20IDs%20Array) (.DeviceID (Utilities|Struct|BreakFoundMIDIDevice _array_element)))
      (Variables|Default|SetDeviceID (Utilities|Array|Get(acopy) _devices_ids_array (Utilities|Array|LastIndex _devices_ids_array))))))

(fn PrintOutcomingValues
  (Development|PrintString (Utilities|String|ToString(Text) (Utilities|Text|FormatText "ch{channel}note{note} at velocity {velocity}" (Variables|Default|GetChannel) (Variables|Default|GetNote) (Variables|Default|GetVelocity)))))