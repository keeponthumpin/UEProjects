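; Hex tile actor that lights up and animates its height when something overlaps its trigger.
; On BeginPlay it picks a random height and RGB multipliers and creates a dynamic glass material instance.
; On overlap it prints a debug message and runs timelines that drive emissive and color parameters and ease the tile's Z scale between that height and 1, setting the trigger's Z scale above the height.
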(event OnComponentBeginOverlap(HexTrigger)
  (params (OverlappedComponent :type Primitive%20Component%20Object%20Reference) (OtherActor :type Actor%20Object%20Reference) (OtherComp :type Primitive%20Component%20Object%20Reference) (OtherBodyIndex :type Integer) (bFromSweep :type Boolean) (SweepResult :type Hit%20Result%20Structure%20%28by%20ref%29))
  (bind _randomheight (Variables|Default|GetRandomHeight))
  (Development|PrintString "triggered")
  (Utilities|FlowControl|Sequence
    (:then_0
      (bind _newtrack_0 (Timeline|Emissive PlayFromStart)
        (:Update
          (Rendering|Material|SetScalarParameterValue (Variables|Default|GetMaterial) "Emissive" _newtrack_0 :!class /Script/Engine.MaterialInstanceDynamic))))
    (:then_1
      (bind _newtrack_0_2 (Timeline|Color_1 PlayFromStart)
        (:Update
          (Rendering|Material|SetScalarParameterValue (Variables|Default|GetMaterial) "R" (* _newtrack_0_2 (Variables|Default|GetR)) :!class /Script/Engine.MaterialInstanceDynamic))))
    (:then_2
      (bind _newtrack_0_3 (Timeline|Color_2 PlayFromStart)
        (:Update
          (Rendering|Material|SetScalarParameterValue (Variables|Default|GetMaterial) "G" (* _newtrack_0_3 (Variables|Default|GetG)) :!class /Script/Engine.MaterialInstanceDynamic))))
    (:then_3
      (bind _newtrack_0_4 (Timeline|Color_3 PlayFromStart)
        (:Update
          (Rendering|Material|SetScalarParameterValue (Variables|Default|GetMaterial) "B" (* _newtrack_0_4 (Variables|Default|GetB)) :!class /Script/Engine.MaterialInstanceDynamic))))
    (:then_4
      (bind _newtrack_0_5 (Timeline|Timeline_3 Play)
        (:Update
          (Transformation|SetWorldScale3D (Variables|Default|GetHexTile) (Math|Vector|MakeVector 1.0 1.0 (Math|Interpolation|Ease "Linear" _newtrack_0_5 _randomheight 1.0)))
          (Transformation|SetWorldScale3D (Variables|Default|GetHexTrigger) (Math|Vector|MakeVector 1.0 1.0 (+ _randomheight 5.0))))))))

(event EventBeginPlay
  (Utilities|FlowControl|Sequence
    (:then_0
      (Variables|Default|SetRandomHeight (Math|Random|RandomFloatinRange 1.0 1e+01)))
    (:then_1
      (bind _returnvalue (Rendering|Material|CreateDynamicMaterialInstance (Variables|Default|GetHexTile) 0 "/Game/Dynamic/M_glass_inst.M_glass_inst" "None" :!class /Script/Engine.PrimitiveComponent))
      (Variables|Default|SetMaterial _returnvalue))
    (:then_2
      (Variables|Default|SetR (Math|Random|RandomFloatinRange 0.1 1.0))
      (Variables|Default|SetG (Math|Random|RandomFloatinRange 0.1 1.0))
      (Variables|Default|SetB (Math|Random|RandomFloatinRange 0.1 1.0)))))

(fn ConstructionScript)