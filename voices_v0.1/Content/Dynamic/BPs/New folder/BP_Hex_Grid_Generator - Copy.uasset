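; Hex grid generator Blueprint that spawns a GridX by GridY field of actors on BeginPlay.
; Nested loops place each cell using per-axis spacing, shifting odd columns along Y by Offset to form the staggered hex layout.
; When SpawnTestGrid is set, the Construction Script builds the same layout from static mesh components with random Z scale, while the spawned actors keep unit scale.
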(event EventBeginPlay
  (for _index (range 0 (Variables|Default|GetGridX))
    (for _index_2 (range 0 (Variables|Default|GetGridY))
      (Game|SpawnActorfromClass "/Game/Dynamic/BP_Hex_Tile.BP_Hex_Tile_C" (Math|Transform|MakeTransform (Math|Vector|SelectVector (Math|Vector|MakeVector (* _index (Variables|Default|GetSpacingX)) (* _index_2 (Variables|Default|GetSpasingY)) 0.0) (Math|Vector|MakeVector (* _index (Variables|Default|GetSpacingX)) (+ (Variables|Default|GetOffset) (* _index_2 (Variables|Default|GetSpasingY))) 0.0) (== (Math|Integer|%(Integer) _index 2) 0)) "0, 0, 0" (Math|Vector|MakeVector 1.0 1.0 1.0)) "Undefined" "MultiplyWithRoot" 0 0))))

(event Collision|EventActorBeginOverlap
  (params (OtherActor :type Actor%20Object%20Reference)))

(event EventTick
  (params (DeltaSeconds :type Float%20%28single-precision%29)))

(fn ConstructionScript
  (if (Variables|Default|GetSpawnTestGrid)
    (for _index (range 0 (Variables|Default|GetGridX))
      (for _index_2 (range 0 (Variables|Default|GetGridY))
        (bind _returnvalue (AddComponent|AddStaticMeshComponent false (Math|Transform|MakeTransform (Math|Vector|SelectVector (Math|Vector|MakeVector (* _index (Variables|Default|GetSpacingX)) (* _index_2 (Variables|Default|GetSpasingY)) 0.0) (Math|Vector|MakeVector (* _index (Variables|Default|GetSpacingX)) (+ (Variables|Default|GetOffset) (* _index_2 (Variables|Default|GetSpasingY))) 0.0) (== (Math|Integer|%(Integer) _index 2) 0)) "0, 0, 0" "1.000000,1.000000,1.000000")))
        (Transformation|SetWorldScale3D _returnvalue (Math|Vector|MakeVector 1.0 1.0 (Math|Random|RandomFloatinRange 1.0 1e+01)))))))