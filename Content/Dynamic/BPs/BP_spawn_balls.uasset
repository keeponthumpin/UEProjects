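; BP_spawn_balls spawns a diagonal row of BP_Bounce actors, each wired to a MIDI output with its own note.
; On BeginPlay it finds the MIDI device matching DeviceName, creates an output controller, and records available device names.
; It then spawns the balls stepped along X and Z, passing each the controller, a rising note, fixed velocity and debug flag.
; DeviceNameChanged reruns only the MIDI setup.
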(event Custom|DeviceNameChanged
  (CallFunction|MIDIOutputcontrollerSetup))

(event EventBeginPlay
  (bind _spawn_transform (Variables|Default|GetSpawn%20Transform))
  (bind (_location _rotation _scale) (Math|Transform|BreakTransform _spawn_transform))
  (bind (_x _y _z) (Math|Vector|BreakVector _location))
  (Utilities|FlowControl|Sequence
    (:then_0
      (CallFunction|MIDIOutputcontrollerSetup))
    (:then_1
      (for _index (range 0 (Variables|Default|GetAmount))
        (bind _returnvalue (Game|SpawnActorfromClass "/Game/Dynamic/BPs/BP_Bounce.BP_Bounce_C" (Math|Transform|MakeTransform (Math|Vector|MakeVector (+ _x (* _index (Variables|Default|GetDistance))) _y (+ _z (* _index (Variables|Default|GetDistance)))) _rotation _scale) "Undefined" "MultiplyWithRoot" 0 0))
        (Variables|/Game/Dynamic/BPs/BP_Bounce.BP_Bounce_C|SetPrintValues _returnvalue (Variables|Default|GetDebug%20Output))
        (Variables|/Game/Dynamic/BPs/BP_Bounce.BP_Bounce_C|SetMidiDeviceOutput _returnvalue (Variables|Default|GetMidi%20Device%20Output))
        (Variables|/Game/Dynamic/BPs/BP_Bounce.BP_Bounce_C|SetNote _returnvalue (+ (* _index 15) 33))
        (Variables|/Game/Dynamic/BPs/BP_Bounce.BP_Bounce_C|SetVelocity _returnvalue 120)))))

(fn ConstructionScript)

(fn MIDIOutputcontrollerSetup
  (bind _devices_ids_array (Variables|Default|GetDevices%20IDs%20Array))
  ;[1 1 1] 1. Find all of the devices. 2.Find device which name matches the midi output we are using. 3. Setup MIDI Output Controller with device ID from the step 2.
  (bind _outmididevices (Class|MIDIDeviceManager|FindMIDIDevices))
  (for _array_element _outmididevices
    (Utilities|FlowControl|Sequence
      (:then_0
        (if (Utilities|Enum|Equal(Enum) (.DeviceName (Utilities|Struct|BreakFoundMIDIDevice _array_element)) (Variables|Default|GetDeviceName))
          (Utilities|Array|Add _devices_ids_array (.DeviceID (Utilities|Struct|BreakFoundMIDIDevice _array_element)))
          (bind _output_get (Variables|Default|SetDevice%20ID (Utilities|Array|Get(acopy) _devices_ids_array (Utilities|Array|LastIndex _devices_ids_array))))
          (bind _returnvalue (Class|MIDIDeviceManager|CreateMIDIDeviceOutputController _output_get))
          (Utilities|IsValid _returnvalue
            (:Is%20Valid
              (Variables|Default|SetMidi%20Device%20Output _returnvalue)))))
      (:then_1
        (Utilities|Array|Add (Variables|Default|GetDevices%20Array) (Utilities|String|ToString(Text) (Utilities|Text|FormatText "{Device name} " (.DeviceName (Utilities|Struct|BreakFoundMIDIDevice _array_element)))))))))